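; TDdoor_BP is a door that slides up automatically when a character enters its collision volume and lowers again when the character leaves.
; Overlap begin and end events play and reverse the DoorOpen timeline, which lerps the Door component's relative Z position between closed and raised.
; Characters are recognized by checking whether the overlapping actor's display name contains "character", rather than by casting to a class.
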(event OnComponentEndOverlap(Collision)
  (params (OverlappedComponent :type Primitive%20Component%20Object%20Reference) (OtherActor :type Actor%20Object%20Reference) (OtherComp :type Primitive%20Component%20Object%20Reference) (OtherBodyIndex :type Integer))
  (if (Utilities|String|Contains (Utilities|GetDisplayName OtherActor) "character")
    (bind _newtrack_0 (Timeline|DoorOpen Reverse)
      (:Update
        (Transformation|SetRelativeLocation (Variables|Default|GetDoor) (Math|Vector|Lerp(Vector) "0, 0,37.500000" "0, 0,200.000000" _newtrack_0) false false)))))

(event OnComponentBeginOverlap(Collision)
  (params (OverlappedComponent :type Primitive%20Component%20Object%20Reference) (OtherActor :type Actor%20Object%20Reference) (OtherComp :type Primitive%20Component%20Object%20Reference) (OtherBodyIndex :type Integer) (bFromSweep :type Boolean) (SweepResult :type Hit%20Result%20Structure%20%28by%20ref%29))
  (if (Utilities|String|Contains (Utilities|GetDisplayName OtherActor) "character")
    (bind _newtrack_0 (Timeline|DoorOpen Play)
      (:Update
        (Transformation|SetRelativeLocation (Variables|Default|GetDoor) (Math|Vector|Lerp(Vector) "0, 0,37.500000" "0, 0,200.000000" _newtrack_0) false false)))))

(event EventBeginPlay)

(event Collision|EventActorBeginOverlap
  (params (OtherActor :type Actor%20Object%20Reference)))

(event EventTick
  (params (DeltaSeconds :type Float%20%28single-precision%29)))

(fn ConstructionScript)