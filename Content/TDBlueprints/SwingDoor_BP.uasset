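; Swinging door Blueprint that the player opens and closes with the E key.
; Overlaps on a Box component enable and disable the actor's input for player controller 0, without filtering the overlapping actor.
; E toggles DoorClosed and plays or reverses the OpenCloseDoor timeline, which drives the Door's absolute world yaw.
; Each press also plays the same door sound at the world origin.
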(event OnComponentBeginOverlap(Box)
  (params (OverlappedComponent :type Primitive%20Component%20Object%20Reference) (OtherActor :type Actor%20Object%20Reference) (OtherComp :type Primitive%20Component%20Object%20Reference) (OtherBodyIndex :type Integer) (bFromSweep :type Boolean) (SweepResult :type Hit%20Result%20Structure%20%28by%20ref%29))
  ;[1 1 1] Enable/Disable Input
  (Input|EnableInput (Game|GetPlayerController 0)))

(event OnComponentEndOverlap(Box)
  (params (OverlappedComponent :type Primitive%20Component%20Object%20Reference) (OtherActor :type Actor%20Object%20Reference) (OtherComp :type Primitive%20Component%20Object%20Reference) (OtherBodyIndex :type Integer))
  ;[1 1 1] Enable/Disable Input
  (Input|DisableInput (Game|GetPlayerController 0)))

(event Input|KeyboardEvents|E
  (params (Key :type Key%20Structure :default "None"))
  (:Pressed
    (Audio|PlaySoundatLocation "/Game/TDBlueprints/Sounds/door-1-open.door-1-open" "0, 0, 0" "0, 0, 0" 1.0 1.0 0.0 0 0 0)
    ;[1 1 1] Open/Close Door
    (if (Variables|Default|GetDoorClosed)
      (Variables|Default|SetDoorClosed false)
      (bind _open_close_door (Timeline|Open/Close%20Door Play)
        (:Update
          (Transformation|SetWorldRotation (Variables|Default|GetDoor) (Math|Rotator|MakeRotator 0.0 0.0 _open_close_door) false false)))
      (else
        (Variables|Default|SetDoorClosed true)
        (Timeline|Open/Close%20Door Reverse)))))

(fn ConstructionScript)